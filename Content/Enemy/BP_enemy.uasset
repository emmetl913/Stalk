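; Enemy pawn Blueprint that chases the player and exposes a patrol route and movement speed functions.
; ChasePlayer moves toward the player pawn with AI Move To and calls itself after a short delay, only on success.
; GetPatrolRoute returns the stored route.
; SetMovementSpeed only returns the current walk speed, as its Chase/Roaming speed selection is disconnected and never runs.
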(event Custom|ChasePlayer
  (AI|AIMoveTo self "0, 0, 0" (Game|Player|GetPlayerPawn 0) 15.0 false
    (:OnSuccess
      (Utilities|FlowControl|Delay 2.0)
      (CallFunction|ChasePlayer))))

(event EventBeginPlay)

(fn ConstructionScript)

(fn GetPatrolRoute
  (return (Variables|AI|GetPatrolRoute)))

(fn SetMovementSpeed
  (params (Speed :type E_MovementSpeed%20Enum :default "NewEnumerator0"))
  (return (stale _output_get)))